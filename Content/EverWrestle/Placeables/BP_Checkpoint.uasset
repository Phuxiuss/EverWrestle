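; BP_Checkpoint is a placeable checkpoint that records which players have reached it and flags when all have.
; On overlap it filters for player-interface actors that cast to BP_EverWrestleCharacter and are not yet collected.
; On the server it adds the character to a set and sends that player the checkpoint location through an interface message.
; AllPlayersCollected turns true once the set size reaches the GameState PlayerArray count.
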(event Collision|EventActorBeginOverlap
  (params (OtherActor :type Actor%20Object%20Reference))
  ;[0.15 0.15 1 0.502] Check if all Players collected the Checkpoint
  (Utilities|ValidandImplementsPlayerInterface OtherActor
    (:Implements
      (bind _asbp_ever_wrestle_character (Utilities|Casting|CastToBP_EverWrestleCharacter OtherActor))
      (if (not (Utilities|Set|Contains (Variables|DeathzoneCommunication|GetPlayersCollected) _asbp_ever_wrestle_character))
        (Networking|SwitchHasAuthority
          (:Authority
            (Utilities|FlowControl|Sequence
              (:then_0
                (Utilities|Set|Add (Variables|DeathzoneCommunication|GetPlayersCollected) _asbp_ever_wrestle_character) ; Set doesn't need to be checked if contains entry already
                (if (>= (Utilities|Set|Length (Variables|DeathzoneCommunication|GetPlayersCollected)) (Utilities|Array|Length (Variables|/Script/Engine.GameStateBase|GetPlayerArray (Game|GetGameState))))
                  (Variables|DeathzoneCommunication|SetbAllPlayersCollected true)))
              (:then_1
                (Class|EverWrestleCharacterInterface|SetPlayerCheckpoint(Message) OtherActor (Transformation|GetActorLocation))))))))))

(fn ConstructionScript)