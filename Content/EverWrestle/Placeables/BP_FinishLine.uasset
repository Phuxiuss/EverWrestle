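; Finish line that records arriving EverWrestle characters, awards placement points by arrival order and sets their checkpoint.
; The first arrival starts the GameMode's round timer through a server event.
; Reaching the session's max players sets AllPlayersFinished, whose OnRep requests the round end.
; When the round ends with one finisher, that player gets placement points again; RewardFirstPlace, which grants every placement's points, is never called here.
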(event Custom|Server_PlayerFinished
  ;[0.15 0.15 1 0.502] Handle the Events that occure when a player enters
  (Networking|SwitchHasAuthority
    (:Authority
      (bind _asbp_ever_wrestle_game_mode (Utilities|Casting|CastToBP_EverWrestleGameMode (Game|GetGameMode)))
      (Class|EverWrestleGameMode|StartRoundTimer _asbp_ever_wrestle_game_mode))))

(event Custom|Server_SwitchToScoreboard
  ;[0.15 0.15 1 0.502] Handle the Events that occure when a player enters
  (Networking|SwitchHasAuthority
    (:Authority
      (bind _asbp_ever_wrestle_game_mode (Utilities|Casting|CastToBP_EverWrestleGameMode (Game|GetGameMode)))
      (Class|EverWrestleGameMode|EndRound _asbp_ever_wrestle_game_mode))))

(event Custom|Server_RequestPointsForPlacement
  (params (PlayerToReward :type BP%20Ever%20Wrestle%20Character%20Object%20Reference))
  ;[0.15 0.15 1 0.502] Add Points for the Placement
  (bind _asbp_ever_wrestle_game_mode (Utilities|Casting|CastToBP_EverWrestleGameMode (Game|GetGameMode)))
  (Utilities|ValidandAuthority _asbp_ever_wrestle_game_mode
    (:ValidAuthority
      (Class|EverWrestleGameMode|AddPointsforPlacement _asbp_ever_wrestle_game_mode PlayerToReward (Math|Conversions|ToByte(Integer) (Utilities|Set|Length (Variables|Default|GetPlayerSet)))))))

(event Custom|CheckPlayerScores
  ;[0.15 0.15 1 0.502] Reward only finished player with everyones points
  (if (== (Utilities|Set|Length (Variables|Default|GetPlayerSet)) 1)
    (CallFunction|ServerRequestPointsforPlacement (Utilities|Set|GetItemByIndex (Variables|Default|GetPlayerSet)))))

(event Custom|RewardFirstPlace
  (params (PlayerToReward :type BP%20Ever%20Wrestle%20Character%20Object%20Reference))
  ;[0.15 0.15 1 0.502] Reward only finished player with everyones points
  (bind _asbp_ever_wrestle_game_mode (Utilities|Casting|CastToBP_EverWrestleGameMode (Game|GetGameMode)))
  (Utilities|ValidandAuthority _asbp_ever_wrestle_game_mode
    (:ValidAuthority
      (for _index (range 1 (Utilities|Array|Length (Variables|/Script/Engine.GameStateBase|GetPlayerArray (Game|GetGameState))))
        (Class|EverWrestleGameMode|AddPointsforPlacement _asbp_ever_wrestle_game_mode PlayerToReward (Math|Conversions|ToByte(Integer) _index))))))

(event EventBeginPlay
  ;[0.15 0.15 1 0.502] Reward only finished player with everyones points
  (bind _asbp_ever_wrestle_game_state (Utilities|Casting|CastToBP_EverWrestleGameState (Game|GetGameState)))
  (EventDispatchers|BindEventtoOnRoundEnded _asbp_ever_wrestle_game_state (delegate Custom|CheckPlayerScores)))

(event Collision|EventActorBeginOverlap
  (params (OtherActor :type Actor%20Object%20Reference))
  ;[0.15 0.15 1 0.502] Check the collided object and fire events
  (Utilities|ValidandImplementsPlayerInterface OtherActor
    (:Implements
      (if (Utilities|Set|IsEmpty (Variables|Default|GetPlayerSet))
        (CallFunction|ServerPlayerFinished))
      (bind _asbp_ever_wrestle_character (Utilities|Casting|CastToBP_EverWrestleCharacter OtherActor))
      (if (not (Utilities|Set|Contains (Variables|Default|GetPlayerSet) _asbp_ever_wrestle_character))
        (Utilities|Set|Add (Variables|Default|GetPlayerSet) _asbp_ever_wrestle_character)
        (CallFunction|ServerRequestPointsforPlacement _asbp_ever_wrestle_character)
        (Class|EverWrestleCharacter|SetCheckpoint _asbp_ever_wrestle_character (Transformation|GetActorLocation))
        (bind _sessionresult (Class|AdvancedSessionSubsystem|GetCurrentSession (Subsystems|GetAdvancedSessionSubsystem))
          (:Valid
            (if (>= (Utilities|Set|Length (Variables|Default|GetPlayerSet)) (Class|FindSessionsCallbackProxy|GetMaxPlayers _sessionresult))
              (Variables|Default|SetbAllPlayersFinished true))))))))

(fn ConstructionScript)

(fn OnRepBAllPlayersFinished
  (CallFunction|ServerSwitchtoScoreboard))