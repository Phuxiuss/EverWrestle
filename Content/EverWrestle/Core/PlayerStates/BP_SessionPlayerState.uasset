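; BP_SessionPlayerState is a player state that tracks each player's chosen character and ready status during a session.
; Server events cycle the character index with wraparound and toggle readiness, then ask the cached BP_SessionGameState to check whether all players are ready.
; RepNotify functions broadcast changes through dispatchers and map the index to a character type enum.
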(event Custom|Server_SetNextCharacterIndex
  (params (MaxLength :type Byte))
  ;[0.15 0.15 1 0.502] Change Character Index on Server
  (bind _nextindex (CallFunction|GetNextCharacterIndex MaxLength))
  (Variables|Default|SetCurrentCharacterIndex _nextindex))

(event Custom|Server_ToggleReadyState
  (bind _cachedgamestate (Variables|Default|GetCachedGameState))
  ;[0.15 0.15 1 0.502] Toggle the Ready State of a player on the Server
  (bind _bisready (CallFunction|GetToggledReadyState))
  (Variables|Default|SetbIsReady _bisready)
  (Utilities|IsValid _cachedgamestate
    (:Is%20Valid
      (Default|CheckAllPlayersReady _cachedgamestate))))

(event EventBeginPlay
  ;[0.15 0.15 1 0.502] Set the Cached Variables
  (bind _asbp_session_game_state (Utilities|Casting|CastToBP_SessionGameState (Game|GetGameState)))
  (Variables|Default|SetCachedGameState _asbp_session_game_state))

(fn ConstructionScript)

(fn OnRepCurrentCharacterIndex
  (bind _currentcharacterindex (Variables|Default|GetCurrentCharacterIndex))
  (Default|CallOnCurrentCharacterIndexChanged _currentcharacterindex)
  (Variables|Default|SetCharacterType (Utilities|Enum|ByteToEnumECharacterType _currentcharacterindex)))

(fn OnRepBIsReady
  (Default|CallOnReadyStateChanged (Variables|Default|GetbIsReady)))

(fn GetToggledReadyState
  (return (not (Variables|Default|GetbIsReady))))

(fn GetNextCharacterIndex
  (params (MaxIndex :type Byte))
  (return (Class|KismetMathLibrary|PercentByteByte (+ (Variables|Default|GetCurrentCharacterIndex) 1) MaxIndex)))

(fn GetReadyState
  (return (Variables|Default|GetbIsReady)))