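; BP_SessionGameState is the session GameState that tracks player readiness and handles requests to start the game.
; CheckAllPlayersReady polls PlayerArray through BPI_SessionInterface and broadcasts whether everyone is ready and the player count meets the session maximum.
; Server_RequestGameStart updates the session to stop advertising and presence joins, starts it, then asks BP_SessionGameMode to start the game.
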(event Custom|CheckAllPlayersReady
  ;[0.15 0.15 1 0.502] Check Ready State
  (bind _sessionresult (Class|AdvancedSessionSubsystem|GetCurrentSession (Subsystems|GetAdvancedSessionSubsystem))
    (:Valid
      (bind _allplayersready (CallFunction|GetAllPlayersReady))
      (Default|CallOnStartStateChanged (and _allplayersready (>= (Utilities|Array|Length (Variables|Default|GetPlayerArray)) (Class|FindSessionsCallbackProxy|GetMaxPlayers _sessionresult)))))))

(event Custom|Server_RequestGameStart
  ;[0.15 0.1221 0 0.502] Request the Game Start from the GameMode
  (bind _asbp_session_game_mode (Utilities|Casting|CastToBP_SessionGameMode (Game|GetGameMode)))
  (bind (_numconnections _numprivateconnections _bislan _bisdedicated _ballowinvites _ballowjoininprogress _bisanticheatenabled _builduniqueid _extrasettings) (Class|AdvancedSessionsLibrary|GetSessionSettings)
    (:OnSuccess
      (|UpdateSession _extrasettings _numconnections _numprivateconnections _bislan _ballowinvites false true _bisdedicated false false false
        (:then
          (|StartAdvancedSession
            (:OnSuccess
              (Default|RequestGameStart _asbp_session_game_mode))))))))

(fn ConstructionScript)

(fn GetAllPlayersReady
  (bind _array_element (Utilities|Array|ForEachLoopwithBreak (Variables|Default|GetPlayerArray) :!label _label)
    (:LoopBody
      (if (Utilities|DoesObjectImplementInterface _array_element "/Game/EverWrestle/Core/PlayerStates/BPI_SessionInterface.BPI_SessionInterface_C")
        (bind _bisready (Class|BPISessionInterface|GetReadyState(Message) _array_element))
        (if (not _bisready)
          (LocalVariables|SetbTempAllReady false)
          (goto _label Break))))
    (:Completed
      (return (LocalVariables|GetbTempAllReady)))))